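; Player-controllable tank Blueprint that wires input and components together for aiming, driving and firing.
; BeginPlay hands the barrel and turret to TankAiming and both tracks to TankMovement.
; Aim axes rotate an azimuth gimbal for yaw and a spring arm for pitch, scaled by delta time.
; Movement axes pass intents to TankMovement, Fire input calls Fire, and construction and BeginPlay print debug strings.
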(event `self.ReceiveBeginPlay`
  (`KismetSystemLibrary.PrintString` "SHREK TankBpBegin Play:")
  (`TankAimingComponent.Initialize` (`self.TankAiming`) (`self.Barrel`) (`self.Turret`))
  (`TankMovementComponent.Initialize` (`self.TankMovement`) (`self.LeftTankTrack`) (`self.RightTankTrack`)))

(event `InputAxis|AimAzimuth`
  (params (AxisValue :type "Float (single-precision)"))
  (`SceneComponent.K2_AddLocalRotation` (`self.Azimuth Gimbal`) (`KismetMathLibrary.MakeRotator` 0.0 0.0 (* AxisValue (`GameplayStatics.GetWorldDeltaSeconds`) 100.0)) false false))

(event `InputAction|Fire`
  (params (Key :type "Key Structure"))
  (:`Pressed`
    (`self.Fire`)))

(event `InputAxis|AimElevation`
  (params (AxisValue :type "Float (single-precision)"))
  (`SceneComponent.K2_AddLocalRotation` (`self.SpringArm`) (`KismetMathLibrary.MakeRotator` 0.0 (* AxisValue (`GameplayStatics.GetWorldDeltaSeconds`) 100.0)) false false))

(event `InputAxis|MoveForward`
  (params (AxisValue :type "Float (single-precision)"))
  (`TankMovementComponent.IntendMoveForward` (`self.TankMovement`) AxisValue))

(event `InputAxis|TurnRight`
  (params (AxisValue :type "Float (single-precision)"))
  (`TankMovementComponent.IntendTurnRight` (`self.TankMovement`) AxisValue))

(fn `UserConstructionScript`
  (`KismetSystemLibrary.PrintString` "SHREK TankBP Construct:"))